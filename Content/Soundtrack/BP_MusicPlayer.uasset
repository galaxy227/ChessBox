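; Music player Blueprint that cycles endlessly through a soundtrack from a random starting point.
; BeginPlay creates a quiet, persistent 2D audio component and fills a seven-slot song array, skipping index 3 and writing Song_8 to index 7, beyond the resized length.
; Tick polls the component and, whenever it is not playing, advances the index with wraparound, then sets and plays that song.
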(event EventBeginPlay
  (bind _song_array (Variables|Default|GetSong%20Array))
  (bind _returnvalue (Audio|CreateSound2D "/Game/Chess_Dir/Audio/click.click" 1.0 1.0 0.0 0 true false))
  (bind _output_get (Variables|Default|SetMusicComponent _returnvalue))
  (Audio|Components|Audio|SetVolumeMultiplier _output_get 0.1 :!class /Script/Engine.AudioComponent)
  (bind _output_get_2 (Variables|Default|SetSongAmount 7))
  (Variables|Default|SetCurrentSongIndex (Math|Random|RandomIntegerinRange 0 (- _output_get_2 1)))
  (Utilities|Array|Resize _song_array _output_get_2)
  (Utilities|Array|SetArrayElem _song_array 0 "/Game/Soundtrack/song_1.song_1")
  (Utilities|Array|SetArrayElem _song_array 1 "/Game/Soundtrack/song_2.song_2")
  (Utilities|Array|SetArrayElem _song_array 2 "/Game/Soundtrack/song_3.song_3")
  (Utilities|Array|SetArrayElem _song_array 4 "/Game/Soundtrack/song_5.song_5")
  (Utilities|Array|SetArrayElem _song_array 5 "/Game/Soundtrack/song_6.song_6")
  (Utilities|Array|SetArrayElem _song_array 6 "/Game/Soundtrack/song_7.song_7")
  (Utilities|Array|SetArrayElem _song_array 7 "/Game/Soundtrack/song_8.song_8"))

(event EventTick
  (params (DeltaSeconds :type Float%20%28single-precision%29))
  (bind _musiccomponent (Variables|Default|GetMusicComponent))
  (bind _song_array (Variables|Default|GetSong%20Array))
  (bind _musiccomponent_2 (Variables|Default|GetMusicComponent))
  (if (Utilities|IsValid _musiccomponent)
    (if (not (Audio|Components|Audio|IsPlaying _musiccomponent)) ; Is Playing
      (if (>= (+ (Variables|Default|GetCurrentSongIndex) 1) (Utilities|Array|Length _song_array)) ; Is Exceed Array
        (Variables|Default|SetCurrentSongIndex 0)
        (else
          (Variables|Default|SetCurrentSongIndex (+ (Variables|Default|GetCurrentSongIndex) 1))))
      (Audio|Components|Audio|SetSound _musiccomponent_2 (Utilities|Array|Get(acopy) _song_array (Variables|Default|GetCurrentSongIndex)))
      (Audio|Components|Audio|Play _musiccomponent_2 0.0))))

(fn ConstructionScript)