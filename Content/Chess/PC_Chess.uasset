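; PC_Chess is the chess player controller, which handles pause menu input.
; On BeginPlay it adds the IMC_Chess Enhanced Input mapping context.
; Each IA_Pause press toggles IsPauseOpen, but the branch condition is fixed to true, so it always creates and adds a new WBP_Pause widget.
; Nothing here removes the widget or pauses the game, and the "NO PAUSE" branch is unreachable.
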(event Input|EnhancedActionEvents|EnhancedInputActionIA_Pause
  (params (ActionValue :type Boolean) (ElapsedSeconds :type Float%20%28double-precision%29) (TriggeredSeconds :type Float%20%28double-precision%29) (InputAction :type Input%20Action%20Object%20Reference :default "/Game/Chess/IA_Pause.IA_Pause"))
  (:Started
    (Variables|Default|SetIsPauseOpen (not (Variables|Default|GetIsPauseOpen)))
    (if true
      (bind _returnvalue (UserInterface|CreateWidget "/Game/Chess/WBP_Pause.WBP_Pause_C" (Game|GetPlayerController 0)))
      (UserInterface|Viewport|AddtoViewport _returnvalue 0)
      (Development|PrintString "PAUSE")
      (else
        (Development|PrintString "NO PAUSE")))))

(event EventBeginPlay
  (Variables|Default|SetIsPauseOpen false)
  (Input|AddMappingContext (PlayerController|LocalPlayerSubsystems|GetEnhancedInputLocalPlayerSubsystem self) "/Game/Chess/IMC_Chess.IMC_Chess" 0 (Utilities|Struct|MakeModifyContextOptions true false false)))

(fn ConstructionScript)