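; BP_TurnReview holds an integer-key snapshot of the chess board, one array entry per square.
; On BeginPlay it sizes the array to the board size squared and fills it with -1.
; SetIntegerKeyIndex walks the board's cubes and encodes each valid piece's player and piece type as a key at that cube's index.
; Cubes without a piece keep their previous value, as only BeginPlay writes -1.
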(event EventBeginPlay
  (bind _integer_key_index (Variables|Default|GetInteger%20Key%20Index))
  (bind _dimension (CallFunction|GetBoardSize))
  (Utilities|Array|Resize _integer_key_index (* _dimension _dimension))
  (for (_ _array_index) _integer_key_index
    (Utilities|Array|SetArrayElem _integer_key_index _array_index -1)))

(fn ConstructionScript)

(fn SetIntegerKeyIndex
  (params (Board :type BP%20Board%20Object%20Reference))
  (for (_array_element _array_index) (Variables|/Game/Chess_Dir/Board/BP_Board.BP_Board_C|GetCubes Board)
    (if (Utilities|IsValid (Variables|/Game/Chess_Dir/Board/BP_Cube.BP_Cube_C|GetPiece _array_element)) ; Is Piece Exist
      (bind _integer_key (CallFunction|VisualPiecetoIntegerKey (Variables|/Game/Chess_Dir/Piece/BP_Piece.BP_Piece_C|GetPlayer%20Type (Variables|/Game/Chess_Dir/Board/BP_Cube.BP_Cube_C|GetPiece _array_element)) (Variables|/Game/Chess_Dir/Piece/BP_Piece.BP_Piece_C|GetPiece%20Type (Variables|/Game/Chess_Dir/Board/BP_Cube.BP_Cube_C|GetPiece _array_element))))
      (Utilities|Array|SetArrayElem (Variables|Default|GetInteger%20Key%20Index) _array_index _integer_key)))
  (return))