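; PC_Chess is the player controller for the chess game, handling input setup and the pause menu.
; On BeginPlay, the local controller adds the IMC_Chess Enhanced Input mapping context.
; IA_Pause toggles a flag that either creates and shows a new WBP_Pause widget with the mouse cursor, or removes it and hides the cursor.
; The toggle changes only the UI and cursor, without pausing the game or switching input mode.
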(event Input|EnhancedActionEvents|EnhancedInputActionIA_Pause
  (params (ActionValue :type Boolean) (ElapsedSeconds :type Float%20%28double-precision%29) (TriggeredSeconds :type Float%20%28double-precision%29) (InputAction :type Input%20Action%20Object%20Reference :default "/Game/Chess_Dir/IA_Pause.IA_Pause"))
  (:Started
    (bind _output_get (Variables|Default|SetIsPauseOpen (not (Variables|Default|GetIsPauseOpen))))
    (if _output_get
      (bind _returnvalue (UserInterface|CreateWidget "/Game/Chess_Dir/WBP_Pause.WBP_Pause_C" (Game|GetPlayerController 0)))
      (bind _output_get_2 (Variables|Default|SetWBP_Pause _returnvalue))
      (UserInterface|Viewport|AddtoViewport _output_get_2 0)
      (Variables|Default|SetbShowMouseCursor true)
      (else
        (Widget|RemovefromParent (Variables|Default|GetWBP_Pause))
        (Variables|Default|SetbShowMouseCursor false)))))

(event EventBeginPlay
  (if (Pawn|IsLocalController)
    (Variables|Default|SetIsPauseOpen false)
    (Input|AddMappingContext (PlayerController|LocalPlayerSubsystems|GetEnhancedInputLocalPlayerSubsystem self) "/Game/Chess_Dir/IMC_Chess.IMC_Chess" 0 "(bIgnoreAllPressedKeysUntilRelease=True,bForceImmediately=False,bNotifyUserSettings=False)")))

(fn ConstructionScript)