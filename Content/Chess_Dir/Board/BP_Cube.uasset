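; BP_Cube is a single chessboard square that colors itself light or dark and reports cursor hover.
; On BeginPlay it derives its type from the parity of its X and Y coordinates, then looks up the matching color.
; RepNotify variables apply that color through a dynamic material instance on the cube mesh.
; Collider cursor events pass the square's coordinates and hover state to the local player's PS_Chess player state.
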(event OnBeginCursorOver(Collider)
  (params (TouchedComponent :type Primitive%20Component%20Object%20Reference))
  (bind _returnvalue (Game|GetPlayerController 0))
  (Utilities|Casting|CastToPC_Chess _returnvalue)
  (bind _asps_chess (Utilities|Casting|CastToPS_Chess (Variables|/Script/Engine.Controller|GetPlayerState _returnvalue)))
  (Default|SetHoverCube _asps_chess (Variables|Default|GetX) (Variables|Default|GetY))
  (Default|SetIsHovering _asps_chess true))

(event OnEndCursorOver(Collider)
  (params (TouchedComponent :type Primitive%20Component%20Object%20Reference))
  (bind _returnvalue (Game|GetPlayerController 0))
  (Utilities|Casting|CastToPC_Chess _returnvalue)
  (bind _asps_chess (Utilities|Casting|CastToPS_Chess (Variables|/Script/Engine.Controller|GetPlayerState _returnvalue)))
  (Default|SetIsHovering _asps_chess false))

(event EventBeginPlay
  (Utilities|SetCubeType)
  (Utilities|SetCubeColor))

(fn ConstructionScript)

(fn OnRepCurrentColor
  (if (Utilities|IsValid (Variables|Default|GetMat_Cube_Instance))
    _
    (else
      (bind _returnvalue (Rendering|Material|CreateDynamicMaterialInstance (Rendering|Material|GetMaterial (Variables|Default|GetCube) 0) "None" "None" :!class /Script/Engine.KismetMaterialLibrary))
      (Variables|Default|SetMat_Cube_Instance _returnvalue)))
  (Rendering|Material|SetVectorParameterValue (Variables|Default|GetMat_Cube_Instance) "Color" (Variables|Default|GetCurrent%20Color) :!class /Script/Engine.MaterialInstanceDynamic)
  (return))

(fn OnRepMatCubeInstance
  (Rendering|Material|SetMaterial (Variables|Default|GetCube) 0 (Variables|Default|GetMat_Cube_Instance))
  (return))