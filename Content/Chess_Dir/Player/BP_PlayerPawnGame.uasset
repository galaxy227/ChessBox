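; BP_PlayerPawnGame is the player pawn for the chess game, providing each player's camera view of the match.
; On BeginPlay it activates its Camera and moves itself to StartingPosition.
; It retries the PlayerState cast to PS_Chess after a short Delay until it succeeds, then yaws the pawn 180 degrees if PlayerType marks the black player.
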(event EventBeginPlay
  (bind _returnvalue (Transformation|GetActorRotation))
  (Components|Activation|SetActive (Variables|Default|GetCamera) true false)
  (Transformation|SetActorLocation self (Variables|Default|GetStarting%20Position) false false)
  ;[0.5 1 1] Set Rotation for Black Player
  (bind _asps_chess (Utilities|Casting|CastToPS_Chess (Variables|GetPlayerState) :!label _label)
    (:then
      (if (Utilities|Enum|Equal(Enum) (Variables|/Game/Chess_Dir/Player/PS_Chess.PS_Chess_C|GetPlayer%20Type _asps_chess) "NewEnumerator1")
        (Transformation|SetActorRotation (Math|Rotator|MakeRotator (.roll _returnvalue) (.pitch _returnvalue) 1.8e+02))))
    (:CastFailed
      (Utilities|FlowControl|Delay 0.01)
      (goto _label))))

(fn ConstructionScript)