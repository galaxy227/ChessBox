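; Game mode for a chess game that assigns each joining player a role as White, Black or spectator.
; On PostLogin, Init Player gets the player's chess player state and fills the first empty seat on the chess game state, White before Black.
; Once both seats are taken, later players join the spectator list.
; Each assignment also sets the PlayerType enum on that player's state.
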(event EventBeginPlay)

(event EventPostLogin
  (params (NewPlayer :type Player%20Controller%20Object%20Reference))
  (Utilities|InitPlayer NewPlayer))

(fn ConstructionScript)