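; BP_Cube is a single chessboard square that picks its light or dark type from the parity of its X and Y at BeginPlay.
; Cursor hover reports its coordinates to PS_Chess, and releasing a click asks PC_Chess to create a piece if IsPlayer passes.
; SetNewColor maps a status to a shade for the square type.
; RepNotifies apply that color through a dynamic material instance.
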(event OnBeginCursorOver(Collider)
  (params (TouchedComponent :type Primitive%20Component%20Object%20Reference))
  (bind _asps_chess (Utilities|Casting|CastToPS_Chess (Variables|/Script/Engine.Controller|GetPlayerState (Game|GetPlayerController 0)))) ; Get Player State
  (Default|SetHoverCube _asps_chess (Variables|Default|GetX) (Variables|Default|GetY)))

(event OnReleased(Collider)
  (params (TouchedComponent :type Primitive%20Component%20Object%20Reference) (ButtonReleased :type Key%20Structure :default "None"))
  (bind _aspc_chess (Utilities|Casting|CastToPC_Chess (Game|GetPlayerController 0)))
  (bind _is_player (Default|IsPlayer _aspc_chess))
  (if _is_player
    (Default|CallCreatePiece _aspc_chess)))

(event EventBeginPlay
  (Utilities|SetCubeType))

(fn ConstructionScript)

(fn SetNewColor
  (params (Status%20Type :type Enum_Cube_Status%20Enum :default "NewEnumerator0"))
  (bind (_light_color _dark_color) (CallFunction|StatustoColor Status%20Type))
  (if (Utilities|Enum|Equal(Enum) (Variables|Default|GetCube%20Type) "NewEnumerator0")
    (Variables|Default|SetCurrent%20Color _light_color)
    (else
      (Variables|Default|SetCurrent%20Color _dark_color)))
  (return))

(fn OnRepCurrentColor
  (if (Utilities|IsValid (Variables|Default|GetMat_Cube_Instance))
    _
    (else
      (bind _returnvalue (Rendering|Material|CreateDynamicMaterialInstance (Rendering|Material|GetMaterial (Variables|Default|GetCube) 0) "None" "None" :!class /Script/Engine.KismetMaterialLibrary))
      (Variables|Default|SetMat_Cube_Instance _returnvalue)))
  (Rendering|Material|SetVectorParameterValue (Variables|Default|GetMat_Cube_Instance) "Color" (Variables|Default|GetCurrent%20Color) :!class /Script/Engine.MaterialInstanceDynamic)
  (return))

(fn StatustoColor
  (params (Status :type Enum_Cube_Status%20Enum :default "NewEnumerator0"))
  (switch Utilities|FlowControl|Switch|SwitchonEnum_Cube_Status Status
    (:NewEnumerator0
      (return "(R=1.000000,G=1.000000,B=1.000000,A=1.000000)" ""))
    (:NewEnumerator1
      (return "(R=1.000000,G=1.000000,B=1.000000,A=1.000000)" ""))
    (:NewEnumerator2
      (return "(R=0.500000,G=0.500000,B=1.000000,A=1.000000)" "(R=0.000000,G=0.000000,B=0.250000,A=1.000000)"))))

(fn OnRepMatCubeInstance
  (Rendering|Material|SetMaterial (Variables|Default|GetCube) 0 (Variables|Default|GetMat_Cube_Instance))
  (return))