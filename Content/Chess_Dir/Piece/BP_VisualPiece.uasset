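; BP_VisualPiece is the visual representation of a chess piece, set up on BeginPlay from its piece type and player type.
; It picks the static mesh for the piece type, then creates a dynamic material instance tinted with the color for its side.
; When the local controller's PS_Chess plays Black, the mesh is yawed 180 degrees, whichever side the piece belongs to.
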(event EventBeginPlay
  (bind _returnvalue (Game|GetPlayerController 0))
  (bind _visualpiece (Variables|Default|GetVisualPiece))
  (bind _visualpiece_2 (Variables|Default|GetVisualPiece))
  (bind _returnvalue_2 (Transformation|GetWorldRotation _visualpiece))
  ;[0.5 1 1] Mesh
  (switch Utilities|FlowControl|Switch|SwitchonEnum_Piece_Type (Variables|Default|GetPiece%20Type)
    (:NewEnumerator0
      (Components|StaticMesh|SetStaticMesh _visualpiece_2 "/Game/Chess_Dir/Mesh/king.king"))
    (:NewEnumerator1
      (Components|StaticMesh|SetStaticMesh _visualpiece_2 "/Game/Chess_Dir/Mesh/queen2.queen2"))
    (:NewEnumerator2
      (Components|StaticMesh|SetStaticMesh _visualpiece_2 "/Game/Chess_Dir/Mesh/rook.rook"))
    (:NewEnumerator3
      (Components|StaticMesh|SetStaticMesh _visualpiece_2 "/Game/Chess_Dir/Mesh/bishop2.bishop2"))
    (:NewEnumerator4
      (Components|StaticMesh|SetStaticMesh _visualpiece_2 "/Game/Chess_Dir/Mesh/knight2.knight2"))
    (:NewEnumerator5
      (Components|StaticMesh|SetStaticMesh _visualpiece_2 "/Game/Chess_Dir/Mesh/pawn2.pawn2")))
  ;[0.5 1 1] Material/Color
  (Rendering|Material|SetMaterial (Variables|Default|GetVisualPiece) 0 "/Game/Chess_Dir/Piece/Mat_VisualPiece.Mat_VisualPiece")
  (bind _returnvalue_3 (Rendering|Material|CreateDynamicMaterialInstance (Rendering|Material|GetMaterial (Variables|Default|GetVisualPiece) 0) "None" "None" :!class /Script/Engine.KismetMaterialLibrary))
  (Variables|Default|SetMat_VisualPiece_Instance _returnvalue_3)
  (switch Utilities|FlowControl|Switch|SwitchonEnum_Player_Type (Variables|Default|GetPlayer%20Type)
    (:NewEnumerator0
      (bind _color (CallFunction|GetColorType "NewEnumerator2"))
      (Rendering|Material|SetVectorParameterValue (Variables|Default|GetMat_VisualPiece_Instance) "Color" _color :!class /Script/Engine.MaterialInstanceDynamic))
    (:NewEnumerator1
      (bind _color_2 (CallFunction|GetColorType "NewEnumerator3"))
      (Rendering|Material|SetVectorParameterValue (Variables|Default|GetMat_VisualPiece_Instance) "Color" _color_2 :!class /Script/Engine.MaterialInstanceDynamic)))
  ;[0.5 1 1] Rotation
  (if (Pawn|IsLocalController _returnvalue)
    (bind _asps_chess (Utilities|Casting|CastToPS_Chess (Variables|/Script/Engine.Controller|GetPlayerState _returnvalue)))
    (if (Utilities|Enum|Equal(Enum) (Variables|/Game/Chess_Dir/Player/PS_Chess.PS_Chess_C|GetPlayer%20Type _asps_chess) "NewEnumerator1")
      (Transformation|SetWorldRotation _visualpiece (Math|Rotator|MakeRotator (.roll _returnvalue_2) (.pitch _returnvalue_2) (+ (.yaw _returnvalue_2) 1.8e+02)) false false))))

(fn ConstructionScript)