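; BP_Piece is a chess piece actor that colors itself by its player type and orients itself for the local player.
; On BeginPlay it names itself, sets CurrentColor for White or Black, and flips its mesh yaw 180 degrees when the local player is Black.
; RepNotify functions propagate the look: the color change creates a dynamic material instance if needed and sets its Color parameter, while the instance change applies it to the mesh.
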(event EventBeginPlay
  (bind _returnvalue (Game|GetPlayerController 0))
  (bind _piece (Variables|Default|GetPiece))
  (bind _returnvalue_2 (Transformation|GetWorldRotation _piece))
  (Variables|Default|SetPiece%20Name "Piece")
  (Utilities|SetColor)
  ;[0.5 1 1] Rotation
  (if (Pawn|IsLocalController _returnvalue)
    (bind _asps_chess (Utilities|Casting|CastToPS_Chess (Variables|/Script/Engine.Controller|GetPlayerState _returnvalue)))
    (if (Utilities|Enum|Equal(Enum) (Variables|/Game/Chess_Dir/Player/PS_Chess.PS_Chess_C|GetPlayer%20Type _asps_chess) "NewEnumerator1")
      (Transformation|SetWorldRotation _piece (Math|Rotator|MakeRotator (.roll _returnvalue_2) (.pitch _returnvalue_2) (+ (.yaw _returnvalue_2) 1.8e+02)) false false))))

(fn ConstructionScript)

(fn OnRepCurrentColor
  (if (Utilities|IsValid (Variables|Default|GetMat_Piece_Instance))
    _
    (else
      (bind _returnvalue (Rendering|Material|CreateDynamicMaterialInstance (Rendering|Material|GetMaterial (Variables|Default|GetPiece) 0) "None" "None" :!class /Script/Engine.KismetMaterialLibrary))
      (Variables|Default|SetMat_Piece_Instance _returnvalue)))
  (Rendering|Material|SetVectorParameterValue (Variables|Default|GetMat_Piece_Instance) "Color" (Variables|Default|GetCurrent%20Color) :!class /Script/Engine.MaterialInstanceDynamic)
  (return))

(fn OnRepMatPieceInstance
  (Rendering|Material|SetMaterial (Variables|Default|GetPiece) 0 (Variables|Default|GetMat_Piece_Instance))
  (return))